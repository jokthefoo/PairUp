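; Football actor that can be passed or shot with mouse clicks while in range, for a co-op football game.
; Any overlap with its Trigger enables the ball's input for player controller 0, and end overlap disables it.
; Left click passes and right click shoots, looping over all OtherChar actors and adding a mesh impulse along each one's forward vector, scaled by PSpeed or SSpeed.
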(event OnComponentBeginOverlap(trigger)
  (params (OverlappedComponent :type Primitive%20Component%20Object%20Reference) (OtherActor :type Actor%20Object%20Reference) (OtherComp :type Primitive%20Component%20Object%20Reference) (OtherBodyIndex :type Integer) (bFromSweep :type Boolean) (SweepResult :type Hit%20Result%20Structure%20%28by%20ref%29))
  ;[1 1 1] Input controll
  (Input|EnableInput (Game|GetPlayerController 0)))

(event OnComponentEndOverlap(trigger)
  (params (OverlappedComponent :type Primitive%20Component%20Object%20Reference) (OtherActor :type Actor%20Object%20Reference) (OtherComp :type Primitive%20Component%20Object%20Reference) (OtherBodyIndex :type Integer))
  ;[1 1 1] Input controll
  (Input|DisableInput (Game|GetPlayerController 0)))

(event Input|MouseEvents|RightMouseButton
  (params (Key :type Key%20Structure))
  ;[1 1 1] Shoot
  (:Pressed
    (bind _outactors (Actor|GetAllActorsOfClass "/Game/ThirdPersonBP/Blueprints/OtherChar.OtherChar_C"))
    (for _array_element _outactors
      (Physics|AddImpulse (Variables|Debug|GetStaticMeshComponent) (* (Transformation|GetActorForwardVector _array_element) (Variables|Default|GetS_Speed)) "None" false)
      (Development|PrintString "Shoot"))))

(event Input|MouseEvents|LeftMouseButton
  (params (Key :type Key%20Structure))
  ;[1 1 1] Pass
  (:Pressed
    (bind _outactors (Actor|GetAllActorsOfClass "/Game/ThirdPersonBP/Blueprints/OtherChar.OtherChar_C"))
    (for _array_element _outactors
      (Physics|AddImpulse (Variables|Debug|GetStaticMeshComponent) (* (Transformation|GetActorForwardVector _array_element) (Variables|Default|GetP_speed)) "None" false)
      (Development|PrintString "Pass"))))

(fn ConstructionScript)